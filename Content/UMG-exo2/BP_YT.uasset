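; Actor that updates a HUD time display and opens two web links, a YouTube video and a Game UI Database page, when shot.
; BeginPlay waits one tick, caches the HUD widget by direct access through a cast of the player's HUD, and initializes its time widget.
; Tick, noted as set to once per second, pushes real-time seconds to that widget.
; The first projectile hit on the mesh launches both URLs through a DoOnce, slightly staggered.
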(event `self.ReceiveBeginPlay`
  ;[0 0 0] Méthode par acces direct. (on note que le tick est reglé pour ne ticker qu'une fois par seconde)
  (`KismetSystemLibrary.DelayUntilNextTick`)
  (bind _ashud_umg_exo_1 (cast `/Game/UMG-exo1/HudUmgExo1` (`PlayerController.GetHUD` (`GameplayStatics.GetPlayerController` 0))))
  (bind _hudref (`/Game/UMG-exo1/HudUmgExo1.hudRef` _ashud_umg_exo_1))
  (`/Engine/EditorBlueprintResources/StandardMacros.IsValid` _hudref
    (:`Is Valid`
      (bind _output_get (set `self.Hud Ref` _hudref))
      (`/Game/UMG-exo1/Interface/IUpdatableText.init` (`/Game/UMG-exo1/WBP_MainScreen.WBP_Time` _output_get)))))

(event `self.ReceiveTick`
  (params (DeltaSeconds :type "Float (single-precision)"))
  ;[0 0 0] Méthode par acces direct. (on note que le tick est reglé pour ne ticker qu'une fois par seconde)
  (bind _hud_ref (`self.Hud Ref`)
    (:`then`
      (message `/Game/UMG-exo1/Interface/IUpdatableText.updateTxt` (`/Game/UMG-exo1/WBP_MainScreen.WBP_Time` _hud_ref) (`KismetStringLibrary.Conv_DoubleToString` (`GameplayStatics.GetRealTimeSeconds`))))
    (:`else`)))

(event `self.StaticMesh.OnComponentHit`
  (params (HitComponent :type "PrimitiveComponent Object Reference") (OtherActor :type "Actor Object Reference") (OtherComp :type "PrimitiveComponent Object Reference") (NormalImpulse :type "Vector Structure") (Hit :type "HitResult Structure (by ref)"))
  (cast `/Game/OverwatchCharacters/Tracer/BP_FirstPersonProjectile` OtherActor)
  (`/Engine/EditorBlueprintResources/StandardMacros.DoOnce` false
    (:`Completed`
      (`KismetSystemLibrary.LaunchURL` "https://www.youtube.com/embed/zUCO9faa-I8?si=TjcJnrrzs09Uc4fF")
      (`KismetSystemLibrary.Delay` 0.2)
      (`KismetSystemLibrary.LaunchURL` "https://www.gameuidatabase.com/gameData.php?id=1808"))))

(fn `UserConstructionScript`)